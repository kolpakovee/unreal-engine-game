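; BP_Traps is a generation helper that spawns spike and moving traps around its X and Y variables at zero height.
; CreateSpikeTrap uses nested random-count loops to scatter BP_SpikeTrap actors in an irregular grid, randomizing spacing and per-axis scale for each spawn.
; CreateMovingTrap spawns a single BP_MovingTrap at X and Y with random per-axis scale.
; BeginPlay and the construction script are empty, and nothing in this Blueprint calls either function.
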(event EventBeginPlay)

(fn ConstructionScript)

(fn CreateSpikeTrap
  (bind _returnvalue (Math|Random|RandomFloatinRange 1.0 5.0))
  (bind _returnvalue_2 (Math|Random|RandomIntegerinRange 1 10))
  (bind _returnvalue_3 (Math|Random|RandomFloatinRange 1e+01 5e+01))
  (for _index (range 0 _returnvalue_2)
    (for _index_2 (range 0 _returnvalue_2)
      (Game|SpawnActorfromClass "/Game/Traps/Blueprints/BP_SpikeTrap.BP_SpikeTrap_C" (Math|Transform|MakeTransform (Math|Vector|MakeVector (+ (* _index _returnvalue_3) (Variables|Default|Getx)) (+ (* _index_2 _returnvalue_3) (Variables|Default|Gety)) 0.0) "0, 0, 0" (Math|Vector|MakeVector _returnvalue _returnvalue _returnvalue)) "Undefined" "MultiplyWithRoot" 0 0))))

(fn CreateMovingTrap
  (bind _returnvalue (Math|Random|RandomFloatinRange 0.5 2.0))
  (Game|SpawnActorfromClass "/Game/Traps/Blueprints/BP_MovingTrap.BP_MovingTrap_C" (Math|Transform|MakeTransform (Math|Vector|MakeVector (Math|Conversions|ToFloat(Integer) (Variables|Default|Getx)) (Math|Conversions|ToFloat(Integer) (Variables|Default|Gety)) 0.0) "0, 0, 0" (Math|Vector|MakeVector _returnvalue _returnvalue _returnvalue)) "Undefined" "MultiplyWithRoot" 0 0))