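; Health pickup actor that applies negative damage to an overlapping actor tagged Player, then destroys itself.
; Healing relies on ApplyDamage with a negative base value, so the receiver's damage handling determines the effect.
; The construction script calls Generate, which attempts to spawn another instance of the same Blueprint at the X and Y variables and a fixed height, with no guard against recursion.
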(event Collision|EventActorBeginOverlap
  (params (OtherActor :type Actor%20Object%20Reference))
  (if (Actor|ActorHasTag OtherActor "Player")
    (Game|Damage|ApplyDamage OtherActor -1e+01 0 0)
    (Actor|DestroyActor)))

(fn ConstructionScript
  (CallFunction|Generate))

(fn Generate
  (Game|SpawnActorfromClass "BP_Health_pickup_C" (Math|Transform|MakeTransform (Math|Vector|MakeVector (Math|Conversions|ToFloat(Integer) (Variables|Default|GetX)) (Math|Conversions|ToFloat(Integer) (Variables|Default|GetY)) 5e+01)) "Undefined" "MultiplyWithRoot" 0 0))