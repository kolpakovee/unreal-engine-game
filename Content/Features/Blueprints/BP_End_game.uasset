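; BP_End_game is an end-of-game trigger actor that responds when an actor tagged Player overlaps it.
; The overlap shows the WB_CompeteGame widget, enables the mouse cursor, switches input to UI only and destroys the trigger.
; A separate Create function spawns a BP_End_game at converted X and Y coordinates with a fixed height.
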(event Collision|EventActorBeginOverlap
  (params (OtherActor :type Actor%20Object%20Reference))
  (bind _returnvalue (Game|GetPlayerController 0))
  (if (Actor|ActorHasTag OtherActor "Player")
    (bind _returnvalue_2 (UserInterface|CreateWidget "/Game/UI/WB_CompeteGame.WB_CompeteGame_C"))
    (UserInterface|Viewport|AddtoViewport _returnvalue_2 0)
    (Variables|/Script/Engine.PlayerController|SetbShowMouseCursor _returnvalue true)
    (Input|SetInputModeUIOnly _returnvalue 0 "DoNotLock" false)
    (Actor|DestroyActor)))

(fn ConstructionScript)

(fn Create
  (Game|SpawnActorfromClass "BP_End_game_C" (Math|Transform|MakeTransform (Math|Vector|MakeVector (Math|Conversions|ToFloat(Integer) (Variables|Default|GetX)) (Math|Conversions|ToFloat(Integer) (Variables|Default|GetY)) 5e+01)) "Undefined" "MultiplyWithRoot" 0 0))