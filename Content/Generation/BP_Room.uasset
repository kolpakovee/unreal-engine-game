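; BP_Room procedurally builds a randomly sized level room when play begins, then increments the game instance's level counter.
; BasicRoomScript, also run at construction, adds instanced bricks for floor, walls and roof.
; It asks existing trap actors to create spike and moving traps, scaled by area and HardCoef.
; It spawns normal and hard doors, or the end point on the final level; hard rooms add extra traps and health pickups.
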(event EventBeginPlay
  (Variables|Default|SetRoomTilesX (Math|Random|RandomIntegerinRange 10 50))
  (Variables|Default|SetRoomTilesY (Math|Random|RandomIntegerinRange 30 60))
  (Variables|Default|SetWallHeight (Math|Random|RandomIntegerinRange 5 10))
  (CallFunction|BasicRoomScript)
  (bind _asbp_game_instance (Utilities|Casting|CastToBP_GameInstance (Game|GetGameInstance)))
  (Default|IncrementCounter _asbp_game_instance))

(fn ConstructionScript
  (CallFunction|BasicRoomScript))

(fn BasicRoomScript
  (Variables|Default|SetSpace (* (Variables|Default|GetRoomTilesX) (Variables|Default|GetRoomTilesY)))
  (CallFunction|GenerateFloor)
  (CallFunction|GenerateTopWall)
  (CallFunction|GenerateBottomWall)
  (CallFunction|GenerateLeftWall)
  (CallFunction|GenerateRightWall)
  (CallFunction|GenerateRoof)
  (CallFunction|GenerateTraps)
  (bind _asbp_game_instance (Utilities|Casting|CastToBP_GameInstance (Game|GetGameInstance)))
  (if (== (Variables|/Game/Levels/BP_GameInstance.BP_GameInstance_C|GetMaxLevel _asbp_game_instance) (Variables|/Game/Levels/BP_GameInstance.BP_GameInstance_C|GetLevelCounter _asbp_game_instance))
    (CallFunction|GenerateFinalPoint)
    (else
      (CallFunction|GenerateDoors)))
  (if (Variables|/Game/Levels/BP_GameInstance.BP_GameInstance_C|GetIsHard _asbp_game_instance)
    (CallFunction|GenerateHealthPickup)))

(fn GenerateFloor
  ;[1 1 1] Generate floor
  (for _index (range 0 (- (Variables|Default|GetRoomTilesX) 1)) ; X
    (for _index_2 (range 0 (- (Variables|Default|GetRoomTilesY) 1)) ; Y
      (Components|InstancedStaticMesh|AddInstance (Variables|Default|GetBrick) (Math|Transform|MakeTransform (Math|Vector|MakeVector (Math|Conversions|ToFloat(Integer) (* _index (Variables|Default|GetMeshWidth))) (Math|Conversions|ToFloat(Integer) (* _index_2 (Variables|Default|GetMeshLength))) 0.0)) false))))

(fn GenerateTopWall
  ;[1 1 1] Generate top wall
  (for _index (range 0 (- (Variables|Default|GetRoomTilesX) 1)) ; X
    (for _index_2 (range 0 (Variables|Default|GetWallHeight)) ; Y
      (Components|InstancedStaticMesh|AddInstance (Variables|Default|GetBrick) (Math|Transform|MakeTransform (Math|Vector|MakeVector (* _index (Variables|Default|GetMeshWidth)) 0.0 (* _index_2 (Variables|Default|GetMeshLength)))) false))))

(fn GenerateLeftWall
  ;[1 1 1] Generate left wall
  (for _index (range 0 (- (Variables|Default|GetRoomTilesY) 1)) ; Y
    (for _index_2 (range 0 (Variables|Default|GetWallHeight)) ; Y
      (Components|InstancedStaticMesh|AddInstance (Variables|Default|GetBrick) (Math|Transform|MakeTransform (Math|Vector|MakeVector 0.0 (* (Variables|Default|GetMeshWidth) _index) (* _index_2 (Variables|Default|GetMeshLength)))) false))))

(fn GenerateRightWall
  ;[1 1 1] Generate right wall
  (for _index (range 0 (- (Variables|Default|GetRoomTilesY) 0)) ; Y
    (for _index_2 (range 0 (Variables|Default|GetWallHeight)) ; Y
      (Components|InstancedStaticMesh|AddInstance (Variables|Default|GetBrick) (Math|Transform|MakeTransform (Math|Vector|MakeVector (* (Variables|Default|GetRoomTilesX) (Variables|Default|GetMeshLength)) (* (Variables|Default|GetMeshWidth) _index) (* _index_2 (Variables|Default|GetMeshLength)))) false))))

(fn GenerateBottomWall
  ;[1 1 1] Generate bottom wall
  (for _index (range 0 (- (Variables|Default|GetRoomTilesX) 1)) ; X
    (for _index_2 (range 0 (Variables|Default|GetWallHeight)) ; Y
      (Components|InstancedStaticMesh|AddInstance (Variables|Default|GetBrick) (Math|Transform|MakeTransform (Math|Vector|MakeVector (* _index (Variables|Default|GetMeshWidth)) (* (Variables|Default|GetRoomTilesY) (Variables|Default|GetMeshWidth)) (* _index_2 (Variables|Default|GetMeshLength)))) false))))

(fn GenerateDoors
  (Game|SpawnActorfromClass "/Game/Generation/BP_Door.BP_Door_C" (Math|Transform|MakeTransform (Math|Vector|MakeVector (- (* (Variables|Default|GetRoomTilesX) (Variables|Default|GetMeshWidth)) 3e+02) (- (* (Variables|Default|GetRoomTilesY) (Variables|Default|GetMeshWidth)) 1e+01) 0.0)) "Undefined" "MultiplyWithRoot" 0 0)
  (bind _returnvalue (Game|SpawnActorfromClass "/Game/Generation/BP_Door.BP_Door_C" (Math|Transform|MakeTransform (Math|Vector|MakeVector (- (* (Variables|Default|GetRoomTilesX) (Variables|Default|GetMeshWidth)) -14.0) (- (* (Variables|Default|GetRoomTilesY) (Variables|Default|GetMeshWidth)) 3e+02) 0.0) "0.000000,90.000000,0.000000") "Undefined" "MultiplyWithRoot" 0 0))
  (bind _output_get (Variables|Default|SetHardDoor _returnvalue))
  (bind _asbp_door (Utilities|Casting|CastToBP_Door _output_get))
  (Variables|/Game/Generation/BP_Door.BP_Door_C|SetIsHard _asbp_door true))

(fn GenerateTraps
  ;[1 1 1] Get hard coef to generate traps
  (bind _asbp_game_instance (Utilities|Casting|CastToBP_GameInstance (Game|GetGameInstance)))
  ;[1 1 1] Generate spike traps
  (for _index (range 0 (+ (Math|Float|Truncate (* (Variables|/Game/Levels/BP_GameInstance.BP_GameInstance_C|GetHard%20Coef _asbp_game_instance) (Variables|Default|GetSpace))) 10))
    (bind _returnvalue (Actor|GetActorOfClass "/Game/Generation/BP_Traps.BP_Traps_C"))
    (Variables|/Game/Generation/BP_Traps.BP_Traps_C|Setx _returnvalue (Math|Random|RandomIntegerinRange 400 (* (Variables|Default|GetRoomTilesX) 100)))
    (Variables|/Game/Generation/BP_Traps.BP_Traps_C|Sety _returnvalue (Math|Random|RandomIntegerinRange 400 (* (Variables|Default|GetRoomTilesY) 100)))
    (Default|CreateSpikeTrap _returnvalue))
  ;[1 1 1] Generate moving traps
  (for _index_2 (range 0 (Math|Float|Truncate (* (Variables|/Game/Levels/BP_GameInstance.BP_GameInstance_C|GetHard%20Coef _asbp_game_instance) (Variables|Default|GetSpace))))
    (bind _returnvalue_2 (Actor|GetActorOfClass "/Game/Generation/BP_Traps.BP_Traps_C"))
    (Variables|/Game/Generation/BP_Traps.BP_Traps_C|Setx _returnvalue_2 (Math|Random|RandomIntegerinRange 500 (- (* (Variables|Default|GetRoomTilesX) 100) 200)))
    (Variables|/Game/Generation/BP_Traps.BP_Traps_C|Sety _returnvalue_2 (Math|Random|RandomIntegerinRange 500 (- (* (Variables|Default|GetRoomTilesY) 100) 200)))
    (Default|CreateMovingTrap _returnvalue_2))
  ;[1 1 1] Generate moving traps if it is a hard room
  (if (Variables|/Game/Levels/BP_GameInstance.BP_GameInstance_C|GetIsHard _asbp_game_instance)
    (for _index_3 (range 0 1)
      (bind _returnvalue_3 (Actor|GetActorOfClass "/Game/Generation/BP_Traps.BP_Traps_C"))
      (Variables|/Game/Generation/BP_Traps.BP_Traps_C|Setx _returnvalue_3 (Math|Random|RandomIntegerinRange 500 (- (* (Variables|Default|GetRoomTilesX) 100) 200)))
      (Variables|/Game/Generation/BP_Traps.BP_Traps_C|Sety _returnvalue_3 (Math|Random|RandomIntegerinRange 500 (- (* (Variables|Default|GetRoomTilesY) 100) 200)))
      (Default|CreateMovingTrap _returnvalue_3))))

(fn GenerateHealthPickup
  (for _index (range 0 (Math|Random|RandomIntegerinRange 0 2))
    (bind _returnvalue (Actor|GetActorOfClass "/Game/Features/Blueprints/BP_Health_pickup.BP_Health_pickup_C"))
    (Variables|/Game/Features/Blueprints/BP_Health_pickup.BP_Health_pickup_C|SetX _returnvalue (Math|Random|RandomIntegerinRange 200 (* (Variables|Default|GetRoomTilesX) 100)))
    (Variables|/Game/Features/Blueprints/BP_Health_pickup.BP_Health_pickup_C|SetY _returnvalue (Math|Random|RandomIntegerinRange 200 (* (Variables|Default|GetRoomTilesY) 100)))
    (Default|Generate _returnvalue)))

(fn GenerateFinalPoint
  (bind _returnvalue (Actor|GetActorOfClass "/Game/Features/Blueprints/BP_End_game.BP_End_game_C"))
  (Variables|/Game/Features/Blueprints/BP_End_game.BP_End_game_C|SetX _returnvalue (- (* (Variables|Default|GetRoomTilesX) 100) 200))
  (Variables|/Game/Features/Blueprints/BP_End_game.BP_End_game_C|SetY _returnvalue (- (* (Variables|Default|GetRoomTilesY) 100) 200))
  (Default|Create _returnvalue))

(fn GenerateRoof
  (bind _meshlength (Variables|Default|GetMeshLength))
  ;[1 1 1] Generate roof
  (for _index (range 0 (- (Variables|Default|GetRoomTilesX) 1)) ; X
    (for _index_2 (range 0 (- (Variables|Default|GetRoomTilesY) 1)) ; Y
      (Components|InstancedStaticMesh|AddInstance (Variables|Default|GetBrick) (Math|Transform|MakeTransform (Math|Vector|MakeVector (Math|Conversions|ToFloat(Integer) (* _index (Variables|Default|GetMeshWidth))) (Math|Conversions|ToFloat(Integer) (* _index_2 _meshlength)) (Math|Conversions|ToFloat(Integer) (* (Variables|Default|GetWallHeight) _meshlength)))) false))))